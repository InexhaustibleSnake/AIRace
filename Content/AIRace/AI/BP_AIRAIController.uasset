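; BP_AIRAIController is an AI controller for the AI Race game that drives its pawn to chase and pick up toys.
; While not chasing a toy, it focuses each tick on the nearest player character.
; When given a target toy, it clears focus and moves to it, picking it up on arrival and retrying the move after a short delay on failure.
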(event `self.ReceiveTick`
  (params (DeltaSeconds :type "Float (single-precision)"))
  (bind _returnvalue (`self.K2_GetPawn`))
  (if (not (`self.ChasingToy`))
    (bind _outactors (`GameplayStatics.GetAllActorsOfClass` "/Game/AIRace/Characters/BP_AIRPlayerCharacter.BP_AIRPlayerCharacter_C"))
    (`self.K2_SetFocus` (`.ReturnValue` (`GameplayStatics.FindNearestActor` (`KismetMathLibrary.SelectVector` (`self.K2_GetActorLocation` _returnvalue) (0.0 0.0 0.0) (`KismetSystemLibrary.IsValid` _returnvalue)) _outactors)))))

(event `self.SetTargetToy`
  (params (TargetToy :type "AIRToy Object Reference"))
  (`parent.SetTargetToy` TargetToy)
  (`self.K2_ClearFocus`)
  (`|AIMoveTo` (`self.K2_GetPawn`) (0.0 0.0 0.0) TargetToy :!label _label
    (:`OnSuccess`
      (`self.PickupToy` TargetToy))
    (:`OnFail`
      (`KismetSystemLibrary.Delay` 0.2)
      (goto _label))))

(fn `UserConstructionScript`)